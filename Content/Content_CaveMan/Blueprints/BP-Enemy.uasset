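; BP-Enemy is an enemy character that detects the player's BP-Caveman and offers movement actions for patrol and combat.
; PawnSensing raises the See flag on a sighting, and a short Delay clears it again.
; SpeedPatrol and SpeedCombat switch the walk speed between slow and fast, and JumpCombat triggers a jump.
; Nothing in this Blueprint reads See or calls those three functions.
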(event `self.PawnSensing.OnSeePawn`
  (params (Pawn :type "Pawn Object Reference"))
  (cast `/Game/Content_CaveMan/Blueprints/BP-Caveman` Pawn)
  (set `self.See?` true)
  (`KismetSystemLibrary.Delay` 0.5)
  (set `self.See?` false))

(fn `JumpCombat`
  (`self.Jump`))

(fn `SpeedCombat`
  (set `CharacterMovementComponent.MaxWalkSpeed` 600.0 (`self.CharacterMovement`)))

(fn `SpeedPatrol`
  (set `CharacterMovementComponent.MaxWalkSpeed` 200.0 (`self.CharacterMovement`)))

(fn `UserConstructionScript`)