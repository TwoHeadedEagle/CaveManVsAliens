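; Behavior tree service that feeds an enemy's vision result into the Blackboard to drive its AI state.
; On activation it sets the default state and records the pawn's location as home.
; Each tick it writes that home vector and reads the BP-Enemy See flag, switching between two states.
; When See is true, it also stores the player controller, not the pawn, as TargetActor, which is never cleared here.
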(event `self.ReceiveActivationAI`
  (params (OwnerController :type "AIController Object Reference") (ControlledPawn :type "Pawn Object Reference"))
  (`BTFunctionLibrary.SetBlackboardValueAsEnum` (`self.StateSelected`) (enumliteral `/Game/Content_CaveMan/Blueprints/AI/AIEnemyStateEnum` "NewEnumerator0"))
  (set `self.HomeVector` (`Actor.K2_GetActorLocation` ControlledPawn)))

(event `self.ReceiveTickAI`
  (params (OwnerController :type "AIController Object Reference") (ControlledPawn :type "Pawn Object Reference") (DeltaSeconds :type "Float (single-precision)"))
  (bind _asbp_enemy (cast `/Game/Content_CaveMan/Blueprints/BP-Enemy` ControlledPawn))
  (`BTFunctionLibrary.SetBlackboardValueAsVector` (`self.HomeSelected`) (`self.HomeVector`))
  (if (`/Game/Content_CaveMan/Blueprints/BP-Enemy.See?` _asbp_enemy)
    (`BTFunctionLibrary.SetBlackboardValueAsEnum` (`self.StateSelected`) (enumliteral `/Game/Content_CaveMan/Blueprints/AI/AIEnemyStateEnum` "NewEnumerator1"))
    (`BTFunctionLibrary.SetBlackboardValueAsObject` (`self.TargetActor`) (`GameplayStatics.GetPlayerController` 0))
    (else
      (`BTFunctionLibrary.SetBlackboardValueAsEnum` (`self.StateSelected`) (enumliteral `/Game/Content_CaveMan/Blueprints/AI/AIEnemyStateEnum` "NewEnumerator0")))))